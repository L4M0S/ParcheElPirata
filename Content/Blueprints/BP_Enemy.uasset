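; Enemy pawn that patrols, chases the player and fires cannonballs, awarding the player a point when destroyed.
; Patrol loops AI moves to random reachable points, changing only X or Y per leg, with random pauses after each arrival.
; Pawn sensing sends it toward the seen character and fires from the right muzzle after a delay.
; Overlapping player-owned cannonballs reduce its health; leftover Move/Turn input handlers and disconnected attack nodes remain.
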(event `self.ReceiveBeginPlay`
  (set `self.StartLocation` (`self.K2_GetActorLocation`))
  (`self.StartPatrolling`))

(event `StartPatrolling`
  (bind _returnvalue (`self.K2_GetActorLocation`))
  (bind _randomlocation (`NavigationSystemV1.K2_GetRandomReachablePointInRadius` _returnvalue (`KismetMathLibrary.RandomFloatInRange` 500.0 1000.0) null null))
  (bind _z (.z _returnvalue))
  (if (`KismetMathLibrary.RandomBool`)
    (`|AIMoveTo` self (`KismetMathLibrary.MakeVector` (.x _randomlocation) (.y _returnvalue) _z) null
      (:`OnSuccess`
        _))
    (else
      (`|AIMoveTo` self (`KismetMathLibrary.MakeVector` (.x _returnvalue) (.y _randomlocation) _z) null
        (:`OnSuccess`
          _))))
  (`KismetSystemLibrary.Delay` (`KismetMathLibrary.RandomFloatInRange` 1.0 3.0))
  (`self.StartPatrolling`))

(event `InputAxis|Move`
  (params (AxisValue :type "Float (single-precision)"))
  ;[1 1 1] Move and Turn
  (`self.AddMovementInput` (`KismetMathLibrary.GetForwardVector` (`KismetMathLibrary.MakeRotator` 0.0 0.0 (.yaw (`self.GetControlRotation`)))) AxisValue))

(event `self.ReceiveActorBeginOverlap`
  (params (OtherActor :type "Actor Object Reference"))
  (bind _asbp_cannon_ball (cast `/Game/Blueprints/BP_CannonBall` OtherActor))
  (cast `/Game/Blueprints/BP_Character` (`/Game/Blueprints/BP_CannonBall.OwnerActor` _asbp_cannon_ball))
  (`self.ApplyDamage` (`/Game/Blueprints/BP_CannonBall.DamageAmount` _asbp_cannon_ball))
  (`self.K2_DestroyActor` OtherActor))

(event `InputAxis|Turn`
  (params (AxisValue :type "Float (single-precision)"))
  ;[1 1 1] Move and Turn
  (`self.AddControllerYawInput` AxisValue))

(event `self.PawnSensing.OnSeePawn`
  (params (Pawn :type "Pawn Object Reference"))
  (bind _asbp_character (cast `/Game/Blueprints/BP_Character` Pawn))
  (`|AIMoveTo` self (`self.K2_GetActorLocation` _asbp_character) null
    (:`then`
      (`KismetSystemLibrary.Delay` 2.0)
      (`|SpawnActorFromClass` "/Game/Blueprints/BP_CannonBall.BP_CannonBall_C" (`SceneComponent.K2_GetComponentToWorld` (`self.RightProjectile`)) "Undefined" "OverrideRootScale" null self null)
      (`AddComponent|NODE_AddAudioComponent-0`))))

(fn `ApplyDamage`
  (params (Amount :type "Float (double-precision)"))
  (set `self.Health` (`KismetMathLibrary.FClamp` (- (`self.Health`) Amount) 0.0 100.0))
  (if (<= (`self.Health`) 0.0)
    (bind _asbp_character (cast `/Game/Blueprints/BP_Character` (`GameplayStatics.GetPlayerCharacter` 0)))
    (set `/Game/Blueprints/BP_Character.Points` (+ (`/Game/Blueprints/BP_Character.Points` _asbp_character) 1) _asbp_character)
    (`self.K2_DestroyActor`)))

(fn `UserConstructionScript`)