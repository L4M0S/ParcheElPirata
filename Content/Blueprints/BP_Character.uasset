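; Player ship character that moves on a plane, fires cannonballs from either side and shows a flipbook chosen in the GameInstance.
; Outside MainMenu it creates HUD, pause-style menu and death widgets; Tick reveals the death screen at zero Health.
; Overlapped loot fills melee, ranged, perk or consumable slots via DT_Items; consumables heal and shield perks absorb damage.
; Melee and Lootear are stubs, ammo decrement is unreachable, and F applies test damage.
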(event `self.ReceiveBeginPlay`
  (bind _returnvalue (`GameplayStatics.GetPlayerController` 0))
  (cast `/Game/Blueprints/BP_GameInstance` (`GameplayStatics.GetGameInstance`))
  (bind _returnvalue_2 (`GameplayStatics.GetCurrentLevelName` true))
  (if (`KismetStringLibrary.NotEqual_StrStr` _returnvalue_2 "MainMenu")
    (bind _returnvalue_3 (`|CreateWidget` "/Game/Widgets/WB_HUD.WB_HUD_C" _returnvalue self))
    (`UserWidget.AddToPlayerScreen` _returnvalue_3 0)
    (bind _returnvalue_4 (`|CreateWidget` "/Game/Widgets/WB_Menu.WB_Menu_C" _returnvalue))
    (bind _output_get (set `self.MenuRef` _returnvalue_4))
    (`UserWidget.AddToPlayerScreen` _output_get 0)
    (`Widget.SetVisibility` _output_get "Hidden")
    (bind _returnvalue_5 (`|CreateWidget` "/Game/Widgets/WB_Death.WB_Death_C" _returnvalue self))
    (bind _output_get_2 (set `self.DeathRef` _returnvalue_5))
    (`UserWidget.AddToViewport` _output_get_2 0)
    (`Widget.SetVisibility` _output_get_2 "Hidden")
    (bind _asbp_game_instance (cast `/Game/Blueprints/BP_GameInstance` (`GameplayStatics.GetGameInstance`)))
    (bind _returnvalue_6 (`PaperFlipbookComponent.SetFlipbook` (`self.Sprite`) (`/Game/Blueprints/BP_GameInstance.CurrentShip` _asbp_game_instance)))
    (if _returnvalue_6
      (`KismetSystemLibrary.PrintString` "correctflipbook"))
    (else
      (`SceneComponent.SetVisibility` (`self.Sprite`) false false))))

(event `InputAction|LeftShoot`
  (params (Key :type "Key Structure"))
  (bind (_rangeweapond_itemid _rangeweapond_amount) (break `/Game/Blueprints/S_PanelItems` (`self.RangeWeapond`)))
  (bind (_rangeweapond_itemid_2 _rangeweapond_amount_2) (break `/Game/Blueprints/S_PanelItems` (`self.RangeWeapond`)))
  ;[1 1 1] RangeWeapon
  (:`Pressed`
    (if (and (!= _rangeweapond_itemid 0) true)
      (`|SpawnActorFromClass` "/Game/Blueprints/BP_CannonBall.BP_CannonBall_C" (`SceneComponent.K2_GetComponentToWorld` (`self.LeftProjectile`)) "Undefined" "OverrideRootScale" null self null)
      (`AddComponent|NODE_AddAudioComponent-0` :!label _label)
      (if (not true)
        (bind _result (`/Engine/EditorBlueprintResources/StandardMacros.DecrementFloat` _rangeweapond_amount_2)
          (:`  `
            (setmembers `/Game/Blueprints/S_PanelItems` :`StructRef` (`self.RangeWeapond`) :`Amount` _result)))))))

(event `InputAxis|Move`
  (params (AxisValue :type "Float (single-precision)"))
  ;[1 1 1] Move and Turn
  (`self.AddMovementInput` (`KismetMathLibrary.GetForwardVector` (`KismetMathLibrary.MakeRotator` 0.0 0.0 (.yaw (`self.GetControlRotation`)))) AxisValue))

(event `InputAction|RightShoot`
  (params (Key :type "Key Structure"))
  (bind (_rangeweapond_itemid _rangeweapond_amount) (break `/Game/Blueprints/S_PanelItems` (`self.RangeWeapond`)))
  ;[1 1 1] RangeWeapon
  (:`Pressed`
    (if (and (!= _rangeweapond_itemid 0) true)
      (`|SpawnActorFromClass` "/Game/Blueprints/BP_CannonBall.BP_CannonBall_C" (`SceneComponent.K2_GetComponentToWorld` (`self.RightProjectile`)) "Undefined" "OverrideRootScale" null self null)
      (goto _label))))

(event `InputAxis|Turn`
  (params (AxisValue :type "Float (single-precision)"))
  ;[1 1 1] Move and Turn
  (`self.AddControllerYawInput` AxisValue))

(event `InputAction|Lootear`
  (params (Key :type "Key Structure"))
  ;[1 1 1] Lootear
  (:`Pressed`
    (if true
      _)))

(event `self.ReceiveActorBeginOverlap`
  (params (OtherActor :type "Actor Object Reference"))
  ;[1 1 1] Lootear
  (bind _asbp_loot (cast `/Game/Blueprints/BP_Loot` OtherActor))
  (bind _returnvalue (`|GetDataTableRow` "/Game/Blueprints/DT_Items.DT_Items" (`KismetStringLibrary.Conv_StringToName` (`KismetStringLibrary.Conv_IntToString` (`/Game/Blueprints/BP_Loot.ItemId` _asbp_loot))))
    (:`then`
      (switch `/Game/Blueprints/E_ItemCategories` (`.Category_20_28965D044C59A4690FB4D69430FF7835` (break `/Game/Blueprints/S_Items` _returnvalue))
        (:`NewEnumerator0`
          (bind _itemid (`/Game/Blueprints/BP_Loot.ItemId` _asbp_loot))
          (bind _ammount (`/Game/Blueprints/BP_Loot.Ammount` _asbp_loot))
          (set `self.MeleeWeapond` (make `/Game/Blueprints/S_PanelItems` _itemid (`KismetMathLibrary.Conv_IntToDouble` _ammount))))
        (:`NewEnumerator1`
          (set `self.RangeWeapond` (make `/Game/Blueprints/S_PanelItems` _itemid (`KismetMathLibrary.Conv_IntToDouble` _ammount)))
          (`KismetSystemLibrary.PrintString` "dfsfs"))
        (:`NewEnumerator2`
          (set `self.Perk` (make `/Game/Blueprints/S_PanelItems` _itemid (`KismetMathLibrary.Conv_IntToDouble` _ammount)))
          (set `self.ShieldActivated?` true))
        (:`NewEnumerator3`
          (set `self.Consumable` (make `/Game/Blueprints/S_PanelItems` _itemid (`KismetMathLibrary.Conv_IntToDouble` _ammount))))
        (:`NewEnumerator4`
          _))
      (`self.K2_DestroyActor` _asbp_loot))))

(event `Key|F`
  (params (Key :type "Key Structure"))
  (:`Pressed`
    (`self.ApplyDamage` 10.0)))

(event `InputAction|Consumable`
  (params (Key :type "Key Structure"))
  (bind _consumable (`self.Consumable`))
  (bind (_consumable_itemid _consumable_amount) (break `/Game/Blueprints/S_PanelItems` (`self.Consumable`)))
  (bind (_itemid _amount) (break `/Game/Blueprints/S_PanelItems` _consumable))
  ;[1 1 1] Consumables
  (:`Pressed`
    (if (> _consumable_amount 0.0)
      (bind _returnvalue (`|GetDataTableRow` "/Game/Blueprints/DT_Items.DT_Items" (`KismetStringLibrary.Conv_StringToName` (`KismetStringLibrary.Conv_IntToString` _consumable_itemid)))
        (:`then`
          (switch `int` _consumable_itemid
            (:`1`
              (set `self.Health` (`KismetMathLibrary.FClamp` (+ (`self.Health`) (`.Value_13_3CE506DB44BC50285B2E3D8BB7F8417E` (break `/Game/Blueprints/S_Items` _returnvalue))) 0.0 100.0))
              (setmembers `/Game/Blueprints/S_PanelItems` :`StructRef` _consumable :`Amount` (- _amount 1.0))
              (if (<= _amount 0.0)
                (set `self.Consumable` (struct))))))))))

(event `InputAction|MeleeWeapond`
  (params (Key :type "Key Structure"))
  ;[1 1 1] MeleeWeapond
)

(event `InputAction|Perk`
  (params (Key :type "Key Structure"))
  (bind (_perk_itemid _perk_amount) (break `/Game/Blueprints/S_PanelItems` (`self.Perk`)))
  ;[1 1 1] Perks
  (:`Pressed`
    (if (> _perk_amount 0.0)
      (`|GetDataTableRow` "/Game/Blueprints/DT_Items.DT_Items" (`KismetStringLibrary.Conv_StringToName` (`KismetStringLibrary.Conv_IntToString` _perk_itemid))
        (:`then`
          (switch `int` _perk_itemid
            (:`3`
              (`/Engine/EditorBlueprintResources/StandardMacros.FlipFlop`
                (:`A`
                  (set `self.ShieldActivated?` true))
                (:`B`
                  (set `self.ShieldActivated?` false))))))))))

(event `Key|P`
  (params (Key :type "Key Structure"))
  (bind _menuref (`self.MenuRef`))
  (:`Pressed`
    (bind _isa (`/Engine/EditorBlueprintResources/StandardMacros.FlipFlop`)
      (:`A`
        (`Widget.SetVisibility` _menuref "Visible"))
      (:`B`
        (`Widget.SetVisibility` _menuref "Hidden")))
    (set `PlayerController.bShowMouseCursor` _isa (`GameplayStatics.GetPlayerController` 0))))

(event `self.ReceiveTick`
  (params (DeltaSeconds :type "Float (single-precision)"))
  (if (<= (`self.Health`) 0.0)
    (`Widget.SetVisibility` (`self.DeathRef`) "Visible")
    (set `PlayerController.bShowMouseCursor` true (`GameplayStatics.GetPlayerController` 0))))

(fn `AddHealth`
  (params (Amount :type "Float (double-precision)"))
  (set `self.Health` (`KismetMathLibrary.FClamp` (+ (`self.Health`) Amount) 0.0 100.0)))

(fn `ApplyDamage`
  (params (Amount :type "Float (double-precision)"))
  (bind _sprite (`self.Sprite`))
  (bind _perk (`self.Perk`))
  (`/Engine/EditorBlueprintResources/StandardMacros.IsValid` self
    (:`Is Valid`
      (if (`self.ShieldActivated?`)
        (bind _structout (setmembers `/Game/Blueprints/S_PanelItems` :`StructRef` _perk :`Amount` (- (`.Amount_9_C9D79CC54F5FF822C251F3A0BEDCAE30` (break `/Game/Blueprints/S_PanelItems` _perk)) Amount)))
        (if (<= (`.Amount_9_C9D79CC54F5FF822C251F3A0BEDCAE30` (break `/Game/Blueprints/S_PanelItems` _structout)) 0.0)
          (set `self.ShieldActivated?` false)
          (set `self.Perk` (struct)))
        (else
          (set `self.Health` (`KismetMathLibrary.FClamp` (- (`self.Health`) Amount) 0.0 100.0))
          (if (<= (`self.Health`) 0.0)
            (set `self.Health` 0.0)
            (`/Engine/EditorBlueprintResources/StandardMacros.IsValid` _sprite
              (:`Is Valid`
                (`ActorComponent.K2_DestroyComponent` _sprite)))))))))

(fn `UserConstructionScript`)